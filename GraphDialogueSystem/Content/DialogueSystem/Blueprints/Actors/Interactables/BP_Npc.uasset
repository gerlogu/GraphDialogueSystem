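; Interactable dialogue NPC whose conversations run as a swappable behavior tree on its AI controller.
; Interacting sets up the player's dialogue camera and HUD and turns the NPC by timeline; further interactions and choices fire dispatchers, and finishing stops the tree.
; A spring-arm camera with matched focus distance frames the dialogue.
; It also supports AI move-to and traces forward each tick to trigger interactables such as doors.
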(event `self.ReceiveTick`
  (params (DeltaSeconds :type "Float (single-precision)"))
  (bind _returnvalue (`self.K2_GetActorLocation`))
  ;[0.01 0.01 0.01] Event Tick
  (bind (_outhit _returnvalue_2) (`KismetSystemLibrary.LineTraceSingle` _returnvalue (+ _returnvalue (* (`self.GetActorForwardVector`) (`self.InteractableCheckRayDistance`))) "TraceTypeQuery1"))
  (if _returnvalue_2
    (bind (_bblockinghit _binitialoverlap _time _distance _location _impactpoint _normal _impactnormal _physmat _hitactor) (`GameplayStatics.BreakHitResult` _outhit))
    (if (`KismetSystemLibrary.DoesImplementInterface` _hitactor "/Game/DialogueSystem/Blueprints/Interfaces/BI_Interactable.BI_Interactable_C")
      (message `/Game/DialogueSystem/Blueprints/Interfaces/BI_Interactable.Interact` _hitactor null))))

(event `/Game/DialogueSystem/Blueprints/Interfaces/BI_DialogableCharacter.SelectChoice`
  (params (ChoiceIndex :type Integer))
  ;[0.01 0.01 0.01] Event Select Choice
  (`self.OnSelectChoice` ChoiceIndex))

(event `/Game/DialogueSystem/Blueprints/Interfaces/BI_Interactable.Interact`
  (params (PlayerRef :type "Actor Object Reference"))
  (bind (_returnvalue_roll _returnvalue_pitch) (`KismetMathLibrary.BreakRotator` (`self.K2_GetActorRotation`)))
  (bind (_returnvalue_roll_2 _returnvalue_pitch_2 _returnvalue_yaw) (`KismetMathLibrary.BreakRotator` (`KismetMathLibrary.FindLookAtRotation` (`self.K2_GetActorLocation`) (`self.K2_GetActorLocation` (`self.Player Ref`)))))
  ;[0.01 0.01 0.01] Event Interact
  (set `self.Player Ref` PlayerRef)
  (if (not (`self.DialogueStarted`))
    (set `self.DialogueStarted` true)
    (`self.SetDialogueCameraLookAtPlayer` (`self.Player Ref`))
    (message `/Game/DialogueSystem/Blueprints/Interfaces/BI_DialogablePlayer.InitDialogueCamera` (`self.Player Ref`))
    (message `/Game/DialogueSystem/Blueprints/Interfaces/BI_DialogablePlayer.InitDialogueHUD` (`self.Player Ref`) (`self.CharacterName`))
    (`AIController.RunBehaviorTree` (`AIBlueprintHelperLibrary.GetAIController` self) (`self.DialogueTree`))
    (set `self.PreDialogueNpcRotation` (`self.K2_GetActorRotation`))
    (bind (_direction _alpha) (`Timeline|T_SetDialogueRotation` :!via `PlayFromStart`)
      (:`Update`
        (`self.K2_SetActorRotation` (`KismetMathLibrary.RLerp` (`self.PreDialogueNpcRotation`) (`KismetMathLibrary.MakeRotator` _returnvalue_roll_2 _returnvalue_pitch _returnvalue_yaw) _alpha true))))
    (else
      (`self.AdvanceDialogue`))))

(event `/Game/DialogueSystem/Blueprints/Interfaces/BI_Interactable.FinishInteract`
  (params (PlayerRef :type "Actor Object Reference"))
  ;[0.01 0.01 0.01] Event Finish Interact
  (set `self.DialogueStarted` false)
  (message `/Game/DialogueSystem/Blueprints/Interfaces/BI_DialogablePlayer.FInishDialogue` PlayerRef)
  (`BrainComponent.StopLogic` (`AIController.BrainComponent` (`AIBlueprintHelperLibrary.GetAIController` self)) "Dialogue Finished"))

(event `/Game/DialogueSystem/Blueprints/Interfaces/BI_DialogableCharacter.SetDialogueTree`
  (params (BehaviorTree :type "BehaviorTree Object Reference"))
  ;[0.01 0.01 0.01] Event Set Dialogue Tree
  (set `self.DialogueTree` BehaviorTree))

(event `/Game/DialogueSystem/Blueprints/Interfaces/BI_DialogableCharacter.MoveTo`
  (params (TargetLocation :type "Vector Structure"))
  ;[0.01 0.01 0.01] Event Move To
  (`|AIMoveTo` self TargetLocation null))

(fn `AdvanceDialogue`
  ;[0.01 0.01 0.01] Advance Dialogue
  (`self.OnContinueDialogue`))

(fn `GetHeadTransform`
  (returns (HeadTransform :type "Transform Structure"))
  ;[0.2135 0.2135 0.2135] Get Bone name
  (return (`SceneComponent.GetSocketTransform` (`self.Mesh`) (`self.HeadName`) "RTS_World")))

(fn `SetDialogueCameraLookAtPlayer`
  (params (PlayerRef :type "Actor Object Reference"))
  (bind (_returnvalue_roll _returnvalue_pitch _returnvalue_yaw) (`KismetMathLibrary.BreakRotator` (`KismetMathLibrary.FindLookAtRotation` (`self.K2_GetActorLocation` PlayerRef) (`self.K2_GetActorLocation`))))
  ;[0.01 0.01 0.01] Set Dialogue Camera Look at Player
  (`SceneComponent.K2_SetWorldRotation` (`self.SpringArm`) (`KismetMathLibrary.MakeRotator` 0.0 0.0 _returnvalue_yaw) false false))

(fn `Speak`
  (params (Sentence :type Text))
  ;[0.01 0.01 0.01] Speak
  (message `/Game/DialogueSystem/Blueprints/Interfaces/BI_DialogablePlayer.UpdateDialogueInfo` (`self.Player Ref`) Sentence))

(fn `UserConstructionScript`
  (bind (_returnvalue_roll _returnvalue_pitch _returnvalue_yaw) (`KismetMathLibrary.BreakRotator` (`KismetMathLibrary.MakeRotFromZ` (`self.GetActorRightVector`))))
  ;[0.01 0.01 0.01] Construction Script
  (set `SpringArmComponent.TargetArmLength` (`self.DialogueCameraArmLength`) (`self.SpringArm`))
  (setmembers `CameraFocusSettings` :`StructRef` (`CineCameraComponent.FocusSettings` (`self.DialogueCamera`)) :`ManualFocusDistance` (`SpringArmComponent.TargetArmLength` (`self.SpringArm`)))
  (`SceneComponent.K2_SetWorldRotation` (`self.SpringArm`) (`KismetMathLibrary.MakeRotator` 0.0 0.0 _returnvalue_yaw) false false))